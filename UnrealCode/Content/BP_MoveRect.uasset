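; BP_MoveRect is an actor that moves its StaticMesh along a looping rectangular path in the relative X-Z plane.
; Each Tick switches on the MoveType enum (Right, UP, Left, Down), steps the X or Z position variable by a fixed amount and applies it as relative location.
; Reaching an edge limit sets the next state, forming a simple state machine.
; Movement is per frame, without delta time, so speed depends on frame rate.
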(event EventBeginPlay)

(event EventTick
  (params (DeltaSeconds :type Float%20%28single-precision%29))
  ;[1 1 1 1 9] 2가지 이상일땐 Enum
  (switch Utilities|FlowControl|Switch|SwitchonEN_MoveType (Variables|Default|GetMoveType)
    (:NewEnumerator0
      ;[1 1 1] 오른쪽으로 이동
      (bind _output_get (Variables|Default|SetX위치 (+ (Variables|Default|GetX위치) 1.0)))
      (Transformation|SetRelativeLocation (Variables|Default|GetStaticMesh) (Math|Vector|MakeVector _output_get 0.0 0.0) false false)
      (if (>= (Variables|Default|GetX위치) 2e+02)
        ;[1 1 1 1 15] 200보다 커지면 어디로 갈건데 ? _ 처음에 가져온 Move Type enum 중에서 'UP'을 세팅해준다.
        (Variables|Default|SetMoveType "NewEnumerator1")))
    (:NewEnumerator1
      ;[1 1 1] Up
      (bind _output_get_2 (Variables|Default|SetZ위치 (+ 1.0 (Variables|Default|GetZ위치))))
      (Transformation|SetRelativeLocation (Variables|Default|GetStaticMesh) (Math|Vector|MakeVector (Variables|Default|GetX위치) 0.0 _output_get_2) false false)
      (if (>= (Variables|Default|GetZ위치) 2e+02)
        (Variables|Default|SetMoveType "NewEnumerator2")))
    (:NewEnumerator2
      ;[1 1 1] 왼쪽으로 이동 - 오른쪽으로 갈때와는 반대(-)로 가야하고, 이때 z값은 전 단계 z위치로 고정
      (bind _output_get_3 (Variables|Default|SetX위치 (- (Variables|Default|GetX위치) 1.0)))
      (Transformation|SetRelativeLocation (Variables|Default|GetStaticMesh) (Math|Vector|MakeVector _output_get_3 0.0 (Variables|Default|GetZ위치)) false false)
      (if (<= (Variables|Default|GetX위치) 0.0)
        (Variables|Default|SetMoveType "NewEnumerator3")))
    (:NewEnumerator3
      ;[1 1 1] Down
      (bind _output_get_4 (Variables|Default|SetZ위치 (- (Variables|Default|GetZ위치) 1.0)))
      (Transformation|SetRelativeLocation (Variables|Default|GetStaticMesh) (Math|Vector|MakeVector (Variables|Default|GetX위치) 0.0 _output_get_4) false false)
      (if (<= (Variables|Default|GetZ위치) 0.0)
        (Variables|Default|SetMoveType "NewEnumerator0")))))

(fn ConstructionScript)