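; BP_ShootingHud is the HUD for the shooting game that creates the HUD widget on BeginPlay and adds it to the viewport.
; It then binds to the HP and magazine update dispatchers on the first player controller's BP_ShootingPlayerState, retrying on a short timer until that cast succeeds.
; Setter functions forward HP, ammo and magazine values to the widget, though no ammo dispatcher is bound here.
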(event EventBeginPlay
  (Utilities|FlowControl|Sequence
    (:then_0
      (bind _returnvalue (UserInterface|CreateWidget "/Game/ShootingGame/Widget/HudWidget.HudWidget_C"))
      (bind _output_get (Variables|Default|SetHudWidget _returnvalue))
      (UserInterface|Viewport|AddtoViewport _output_get 0))
    (:then_1
      (CallFunction|BindMyPlayerState))))

(fn ConstructionScript)

(fn SetHptoWidget
  (params (CurHp :type Float%20%28double-precision%29) (MaxHp :type Float%20%28double-precision%29))
  (Default|SetHp (Variables|Default|GetHudWidget) CurHp MaxHp))

(fn BindMyPlayerState
  (bind _asbp_shooting_player_state (Utilities|Casting|CastToBP_ShootingPlayerState (Variables|/Script/Engine.Controller|GetPlayerState (Game|GetPlayerController 0)))
    (:then
      (EventDispatchers|BindEventtoEventDispatcherUpdateHp _asbp_shooting_player_state (EventDispatchers|CreateEvent :!event SetHptoWidget))
      (EventDispatchers|BindEventtoEventDispatcherUpdateMag _asbp_shooting_player_state (EventDispatchers|CreateEvent :!event SetMagtoWidget)))
    (:CastFailed
      (Utilities|Time|SetTimerbyFunctionName 0 "BindMyPlayerState" 0.01))))

(fn SetAmmotoWidget
  (params (Ammo :type Integer))
  (Default|SetAmmo (Variables|Default|GetHudWidget) Ammo))

(fn SetMagtoWidget
  (params (Mag :type Integer))
  (Default|SetMag (Variables|Default|GetHudWidget) Mag))