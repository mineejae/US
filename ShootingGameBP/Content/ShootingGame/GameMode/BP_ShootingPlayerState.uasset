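; Player state for the shooting game that tracks each player's health and spare magazine count.
; Health starts full on BeginPlay and drops through AddDamage, while AddMag, UseMag and IsCanReload manage the magazines available for reloading.
; Both values use RepNotify functions that fire UpdateHp and UpdateMag event dispatchers, broadcasting changes to any listeners.
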(event EventBeginPlay
  (Variables|Default|SetCurHp 1e+02))

(fn ConstructionScript)

(fn AddDamage
  (params (Damage :type Float%20%28double-precision%29))
  (Variables|Default|SetCurHp (- (Variables|Default|GetCurHp) Damage)))

(fn OnRepCurHp
  (Default|CallEventDispatcherUpdateHp (Variables|Default|GetCurHp) 1e+02))

(fn AddMag
  (Variables|Default|SetMag (+ (Variables|Default|GetMag) 1)))

(fn OnRepMag
  (Default|CallEventDispatcherUpdateMag (Variables|Default|GetMag)))

(fn UseMag
  (if (> (Variables|Default|GetMag) 0)
    (Variables|Default|SetMag (+ (Variables|Default|GetMag) -1))
    (return true)
    (else
      (return false))))

(fn IsCanReload
  (return (> (Variables|Default|GetMag) 0)))