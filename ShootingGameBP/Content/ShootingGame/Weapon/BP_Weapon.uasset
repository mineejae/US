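; Networked rifle weapon actor for the shooting game, handling pickup to the character's weapon socket, physics drop, firing and reloading.
; Trigger and reload events play montages, while separate shoot and reload-complete events let the local player send requests to the server.
; The server requests spend ammo and apply damage via a camera-aimed line trace, or refill ammo using a PlayerState magazine.
; Ammo's OnRep updates the local player's HUD.
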(event Custom|ReqApplyDamage
  (params (Start :type Vector) (End :type Vector))
  (Development|PrintString "(Server)ReqApplyDamage" false true "(R=0.000000,G=0.660000,B=1.000000,A=1.000000)" 6e+01)
  (CallFunction|UseAmmo)
  (bind _outhit (Collision|LineTraceForObjects Start End (Utilities|Array|MakeArray "ObjectTypeQuery1" "ObjectTypeQuery2" "ObjectTypeQuery3" "ObjectTypeQuery4" "ObjectTypeQuery5" "ObjectTypeQuery6") false (Utilities|Array|MakeArray (Variables|Default|GetCharacter)) "Persistent"))
  (bind _as캐릭터 (Utilities|Casting|CastToCharacter (.HitActor (Collision|BreakHitResult _outhit))))
  ;[1 0 0] 이 뒤쪽 실행라인은 실행 안됨
  (Game|Damage|ApplyDamage _as캐릭터 1e+01 (Pawn|GetController (Variables|Default|GetCharacter)) self))

(event Custom|ReqReload
  (Development|PrintString "ReqReload!!!!!" true true "(R=0.000000,G=0.660000,B=1.000000,A=1.000000)" 6e+01)
  (bind _asbp_shooting_player_state (Utilities|Casting|CastToBP_ShootingPlayerState (Variables|/Script/Engine.Pawn|GetPlayerState (Variables|Default|GetCharacter))))
  (bind _isused (Default|UseMag _asbp_shooting_player_state))
  (if _isused
    (Variables|Default|SetAmmo 30)))

(event EventBeginPlay
  (CallFunction|UpdateHUDMyAmmo (Variables|Default|GetAmmo)))

(fn ConstructionScript)

(fn CalcShootStartEndPos
  (bind _returnvalue (Game|GetPlayerCameraManager 0))
  (bind _returnvalue_2 (Transformation|GetActorLocation _returnvalue))
  (bind _returnvalue_3 (Transformation|GetActorRotation _returnvalue))
  (bind _returnvalue_4 (Math|Vector|GetForwardVector _returnvalue_3))
  (return (+ _returnvalue_2 (* _returnvalue_4 (+ (Variables|/Script/Engine.SpringArmComponent|GetTargetArmLength (Actor|GetComponentbyClass (Variables|Default|GetCharacter) "/Script/Engine.SpringArmComponent")) 1e+02))) (+ _returnvalue_2 (* _returnvalue_4 1e+04))))

(fn OnRepAmmo
  (CallFunction|UpdateHUDMyAmmo (Variables|Default|GetAmmo)))

(fn UpdateHUDMyAmmo
  (params (Ammo :type Integer))
  (if (== (Variables|Default|GetCharacter) (Game|GetPlayerCharacter 0))
    (bind _asbp_shooting_hud (Utilities|Casting|CastToBP_ShootingHud (HUD|GetHUD (Game|GetPlayerController 0))))
    (Default|SetAmmotoWidget _asbp_shooting_hud Ammo)))

(fn UseAmmo
  (Variables|Default|SetAmmo (Math|Integer|Clamp(Integer) (- (Variables|Default|GetAmmo) 1) 0 30)))

(fn EventDrop
  (params (Character :type Character%20Object%20Reference))
  (bind _staticmesh (Variables|Default|GetStaticMesh))
  (CallFunction|UpdateHUDMyAmmo)
  (Variables|Default|SetCharacter 0)
  (Transformation|DetachFromComponent _staticmesh "KeepWorld" "KeepWorld" "KeepWorld" true)
  (Collision|SetCollisionEnabled _staticmesh "QueryAndPhysics")
  (Physics|SetSimulatePhysics _staticmesh true)
  (Actor|SetOwner 0)
  (return false))

(fn EventPickup
  (params (Character :type Character%20Object%20Reference))
  (bind _staticmesh (Variables|Default|GetStaticMesh))
  (bind _output_get (Variables|Default|SetCharacter Character))
  (Physics|SetSimulatePhysics _staticmesh false)
  (Collision|SetCollisionEnabled _staticmesh "NoCollision")
  (Transformation|AttachComponentToComponent (Variables|/Script/Engine.Character|GetMesh _output_get) "weapon" "SnapToTarget" "SnapToTarget" "KeepRelative" true)
  (CallFunction|UpdateHUDMyAmmo (Variables|Default|GetAmmo))
  (return false))

(fn EventReload
  (Animation|PlayAnimMontage (Variables|Default|GetCharacter) "/Game/Characters/Mannequins/Animations/InPlace/Rifle_Reload_2_Montage.Rifle_Reload_2_Montage" 1.0 "None")
  (return false))

(fn EventReloadComplate
  (Development|PrintString "EventReloadComplate")
  (if (== (Game|GetPlayerController 0) (Pawn|GetController (Variables|Default|GetCharacter)))
    (CallFunction|ReqReload)
    (return false)))

(fn EventShoot
  (bind (_start _end) (CallFunction|CalcShootStartEndPos))
  (bind _staticmesh (Variables|Default|GetStaticMesh))
  (bind _returnvalue (Transformation|GetSocketTransform _staticmesh "muzzle" "RTS_World"))
  (Effects|SpawnEmitteratLocation "/Game/StarterContent/Particles/P_Explosion.P_Explosion" (.location _returnvalue) (.rotation _returnvalue) "0.200000,0.200000,0.200000")
  (if (== (Game|GetPlayerCharacter 0) (Variables|Default|GetCharacter))
    (Development|PrintString "(Client)ReqApplyDamage" true true "(R=0.000000,G=0.660000,B=1.000000,A=1.000000)" 6e+01)
    (CallFunction|ReqApplyDamage _start _end)
    (return false)))

(fn EventTrigger
  (params (IsPress :type Boolean))
  (Animation|PlayAnimMontage (Variables|Default|GetCharacter) "/Game/Characters/Mannequins/Animations/InPlace/Rifle_ShootOnce_Montage.Rifle_ShootOnce_Montage" 1.0 "None")
  (return false))