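; BP_Weapon_MachineGun is a shooting game weapon that handles automatic fire while the trigger is held.
; EventTrigger calls ShootOnce immediately on press, then repeats it on a short looping timer set by function name until release clears it.
; ShootOnce only plays the rifle shot montage on the Character, with no projectile or damage logic in this graph.
; The default event graph nodes are empty or disabled.
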(event EventBeginPlay
  (|CallParentFunction) ; 지금 이 노드는 비활성 상태입니다. \n핀을 끌어서 다른 노드를 연결하면 활성화됩니다.
)

(event Collision|EventActorBeginOverlap
  (params (OtherActor :type Actor%20Object%20Reference)))

(event EventTick
  (params (DeltaSeconds :type Float%20%28single-precision%29)))

(fn ConstructionScript
  (|CallParentFunction))

(fn ShootOnce
  (Animation|PlayAnimMontage (Variables|Default|GetCharacter) "/Game/Characters/Mannequins/Animations/InPlace/Rifle_ShootOnce_Montage.Rifle_ShootOnce_Montage" 1.0 "None"))

(fn EventTrigger
  (params (IsPress :type Boolean))
  (if IsPress
    (CallFunction|ShootOnce)
    (Utilities|Time|SetTimerbyFunctionName 0 "ShootOnce" 0.1 true)
    (return true)
    (else
      (Utilities|Time|ClearTimerbyFunctionName 0 "ShootOnce")
      (return true))))